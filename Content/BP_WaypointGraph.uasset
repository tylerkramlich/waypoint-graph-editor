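; Waypoint graph actor that links BP_Waypoint actors in the level into a neighbor network.
; BuildGraph gathers every waypoint and line-traces between each pair's top viewpoints on Visibility, adding mutual neighbors when the trace hits the other waypoint within a short range.
; BeginPlay only calls DrawConnections, leaving BuildGraph to be triggered separately.
; An unwired fragment constructs a WaypointConnection between the first two waypoints.
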(event Custom|Build%20Graph
  (bind _outactors (Actor|GetAllActorsOfClass "/WaypointGraphEditor/BP_Waypoint.BP_Waypoint_C"))
  ;[1 1 1] Comment
  (Variables|Default|SetWaypoints _outactors)
  (if true
    (for _array_element _outactors
      (for _array_element_2 _outactors
        (bind _returnvalue (Default|GetTopViewpoint _array_element))
        (bind _returnvalue_2 (Default|GetTopViewpoint _array_element_2))
        (bind _outhit (Collision|LineTraceByChannel _returnvalue _returnvalue_2 "TraceTypeQuery1" true (Utilities|Array|MakeArray _array_element) "None"))
        (if (== (.hitactor _outhit) _array_element_2)
          (if (<= (.distance _outhit) 3e+02)
            (Utilities|Array|AddUnique (Variables|/Script/WaypointGraphEditor.Waypoint|GetNeighbors _array_element) _array_element_2)
            (Utilities|Array|AddUnique (Variables|/Script/WaypointGraphEditor.Waypoint|GetNeighbors _array_element_2) _array_element)))))))

(event EventBeginPlay
  (Class|WaypointGraph|DrawConnections))

(fn ConstructionScript)